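; Openable door actor that swings open and closed when its OpenDoor component fires open and close events.
; A timeline adds an animated yaw angle to the rotation stored at BeginPlay, and closing plays that timeline in reverse.
; An event track on the timeline plays the Doorlock sound at the door's location.
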(event `self.ReceiveBeginPlay`
  (set `self.InitialRotation` (`self.K2_GetActorRotation`)))

(event `self.OpenDoor.OnOpen`
  (bind (_direction _openangle) (`Timeline|Door Swing Timeline` :!label _label)
    (:`Update`
      (`self.K2_SetActorRotation` (`KismetMathLibrary.ComposeRotators` (`self.InitialRotation`) (`KismetMathLibrary.MakeRotator` 0.0 0.0 _openangle))))
    (:`Sound Timing`
      (`GameplayStatics.PlaySoundAtLocation` "/Game/door-lock.door-lock" (`self.K2_GetActorLocation`)))))

(event `self.OpenDoor.OnClose`
  (goto _label :!via `Reverse`))

(fn `UserConstructionScript`)